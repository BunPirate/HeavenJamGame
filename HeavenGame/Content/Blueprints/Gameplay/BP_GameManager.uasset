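; Game manager actor for what appears to be a wave-based tower defense level, owning the enemy path, base health, HUD and game over.
; The construction script builds spline meshes along the path and places start and end markers.
; BeginPlay initializes the healthbar, HUD, currency and wave manager, while SpawnEnemy spawns enemies at the spline start.
; DoDamage reduces base health for one team value, showing death UI and freezing time below zero.
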(event `SetStartAndEnd`
  (bind _spline (`self.Spline`))
  ;[0.499 1 0.3404] Spline Stuff
  (`SceneComponent.K2_SetRelativeLocation` (`self.StartMesh`) (`SplineComponent.GetLocationAtSplinePoint` _spline 0 "Local") false false)
  (`SceneComponent.K2_SetRelativeLocation` (`self.EndMesh`) (`SplineComponent.GetLocationAtSplinePoint` _spline (- (`SplineComponent.GetNumberOfSplinePoints` _spline) 1) "Local") false false))

(event `self.ReceiveBeginPlay`
  (bind _basehealth (`self.BaseHealth`))
  ;[0.3751 1 0.2804] Init Chain
  (bind _asw_healthbar (cast `/Game/Blueprints/UI/W_Healthbar` (`WidgetComponent.GetWidget` (`self.BaseHealthbar`))))
  (bind _output_get (set `self.As W Healthbar` _asw_healthbar))
  (`/Game/Blueprints/UI/W_Healthbar.UpdateHealthBar` _output_get (`KismetMathLibrary.Conv_IntToDouble` (/ _basehealth (`self.BaseMaxHealth`))) (`KismetMathLibrary.Conv_IntToDouble` _basehealth) "Base")
  (`self.CreateHUD`)
  (`/Game/Jake-Towers/BP_Currency.Init_Currency` (`self.BP_Currency`) self)
  (`/Game/Jake-Towers/BP_WaveManager.Init_WaveManager` (`self.BP_WaveManager`) (`self.HUD_UI_Ref`) self "NewEnumerator0"))

(event `SpawnEnemy`
  (bind _returnvalue (`|SpawnActorFromClass` "/Game/Blueprints/Enemies/BP_EnemyBase.BP_EnemyBase_C" (`KismetMathLibrary.MakeTransform` (`SplineComponent.GetLocationAtSplinePoint` (`self.Spline`) 0 "World")) "Undefined" "OverrideRootScale" null null))
  (`/Game/Blueprints/Enemies/BP_EnemyBase.InitEnemy` _returnvalue self))

(event `/Game/Blueprints/Enemies/BPI_Damage.DoDamage`
  (params (Team :type "/Game/Blueprints/Enemies/E_Team Enum" :default "NewEnumerator0") (Damage :type "Float (double-precision)"))
  (bind _basehealth (`self.BaseHealth`))
  (bind _returnvalue (`KismetMathLibrary.FTrunc` (- (`self.BaseHealth`) Damage)))
  ;[1 1 1] Do Damange Interface Stuff
  (if (`|EnumEquality` Team "NewEnumerator1")
    (if (< _returnvalue 0)
      (set `self.BaseHealth` 0)
      (`|ExecutionSequence`
        (:`then_0`
          (`/Game/Blueprints/UI/W_Healthbar.UpdateHealthBar` (`self.As W Healthbar`) (/ _basehealth (`self.BaseMaxHealth`)) (`KismetMathLibrary.Conv_IntToDouble` _basehealth) "Base" :!label _label))
        (:`then_1`
          (`self.Dead`)))
      (else
        (set `self.BaseHealth` _returnvalue)
        (goto _label)))))

(fn `CreateHUD`
  ;[1 1 1] Setup HUD
  (bind _returnvalue (`|CreateWidget` "/Game/Blueprints/UI/HUD_Main.HUD_Main_C"))
  (bind _output_get (set `self.HUD_UI_Ref` _returnvalue))
  (`UserWidget.AddToViewport` _output_get 0))

(fn `Dead`
  ;[1 1 1] Show Death UI
  (`/Game/Blueprints/UI/W_GameOver.Death_ShowUI` (`/Game/Blueprints/UI/HUD_Main.W_GameOver` (`self.HUD_UI_Ref`)))
  ;[1 1 1] Freeze Time
  (`GameplayStatics.SetGlobalTimeDilation` 0.0))

(fn `GetEnemy`
  (returns (EnemyBase :type "/Game/Blueprints/Enemies/BP_EnemyBase Object Reference"))
  (return null))

(fn `UserConstructionScript`
  (bind _spline (`self.Spline`))
  (bind _returnvalue (`SplineComponent.GetNumberOfSplinePoints` (`self.Spline`)))
  (`self.SetStartAndEnd`)
  (for _index (range _returnvalue)
    (if (not (== _index (- _returnvalue 1)))
      (bind _returnvalue_2 (`AddComponent|NODE_AddSplineMeshComponent-1`))
      (bind _returnvalue_3 (+ _index 1))
      (`SplineMeshComponent.SetStartAndEnd` _returnvalue_2 (`SplineComponent.GetLocationAtSplinePoint` _spline _index "Local") (`SplineComponent.GetTangentAtSplinePoint` _spline _index "Local") (`SplineComponent.GetLocationAtSplinePoint` _spline _returnvalue_3 "Local") (`SplineComponent.GetTangentAtSplinePoint` _spline _returnvalue_3 "Local") true))))