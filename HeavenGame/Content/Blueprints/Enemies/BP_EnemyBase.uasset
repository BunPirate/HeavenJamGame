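; Base enemy actor that travels along a spline path and can be damaged and destroyed.
; InitEnemy stores the game manager, takes its spline and sets the mesh collision object type to Destructible.
; Tick advances distance by Speed and moves the root to that spline point without sweeping.
; DoDamage lowers Health only for one team value and calls Die on its health check, while GetEnemy returns the actor itself.
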(event `InitEnemy`
  (params (GameManager :type "/Game/Blueprints/Gameplay/BP_GameManager Object Reference"))
  (bind _output_get (set `self.GameManager` GameManager))
  (set `self.Spline` (`/Game/Blueprints/Gameplay/BP_GameManager.Spline` _output_get))
  (`PrimitiveComponent.SetCollisionObjectType` (`self.EnemyMesh`) "ECC_Destructible"))

(event `self.ReceiveTick`
  (params (DeltaSeconds :type "Float (single-precision)"))
  ;[1 1 1] Move enemy along spline
  (bind _output_get (set `self.ProgressAlongSpline` (+ (`self.ProgressAlongSpline`) (* DeltaSeconds (`self.Speed`)))))
  (`SceneComponent.K2_SetWorldLocation` (`self.DefaultSceneRoot`) (`SplineComponent.GetLocationAtDistanceAlongSpline` (`self.Spline`) _output_get "World") false false))

(event `Die`
  (`self.K2_DestroyActor`))

(event `/Game/Blueprints/Enemies/BPI_Damage.DoDamage`
  (params (Team :type "/Game/Blueprints/Enemies/E_Team Enum" :default "NewEnumerator0") (Damage :type "Float (double-precision)"))
  (bind _returnvalue (- (`self.Health`) Damage))
  ;[1 1 1] Damge enemy
  (if (`|EnumEquality` Team "NewEnumerator0")
    (set `self.Health` _returnvalue)
    (if (<= _returnvalue 0.0)
      (`self.Die`))))

(fn `GetEnemy`
  (returns (EnemyBase :type "/Game/Blueprints/Enemies/BP_EnemyBase Object Reference"))
  (return self))

(fn `UserConstructionScript`)