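; BP_PlayerPawn is the player pawn that handles cursor-based interaction with objects in the level.
; On the Interact input it traces under the cursor, then hides the Build and Sell UI on every BP_BuildingPlot found in the level.
; It then sends an InteractMessage to the hit actor, passing itself, and prints a debug string.
; The all-actors sweep on each click carries an author note that it may hurt performance.
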(event `InputAction|Interact`
  (params (Key :type "Key Structure"))
  (bind (_hitresult _returnvalue) (`PlayerController.GetHitResultUnderCursorByChannel` (`GameplayStatics.GetPlayerController` 0) "TraceTypeQuery1" true))
  (:`Pressed`
    (if _returnvalue
      ;[1 0.2806 0.3104] May Destroy Performance -  Close all open Build/Sell UI Widgets
      (bind _outactors (`GameplayStatics.GetAllActorsOfClass` "/Game/Blueprints/BP_BuildingPlot.BP_BuildingPlot_C"))
      (for _array_element _outactors
        (`SceneComponent.SetVisibility` (`/Game/Blueprints/BP_BuildingPlot.BuildUI` _array_element) false false)
        (`SceneComponent.SetVisibility` (`/Game/Blueprints/BP_BuildingPlot.SellUI` _array_element) false false))
      (message `/Game/Blueprints/BPI_Interact.Interact` (`.HitActor` (`GameplayStatics.BreakHitResult` _hitresult)) self)
      (`KismetSystemLibrary.PrintString` "Interacted"))))

(fn `UserConstructionScript`)