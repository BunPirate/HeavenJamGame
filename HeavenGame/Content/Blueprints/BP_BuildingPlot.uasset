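; BP_BuildingPlot is a tower-defense build spot where the player builds, upgrades or sells a tower.
; BeginPlay hides and initializes its three menu widget components, handing them plot or game manager references.
; Interact closes build and sell menus on all plots, then, unless the game has ended, shows menus matching occupancy and tower level.
; SpawnTower creates and initializes a BP_TowersMain, while SellTower triggers its explosion and frees the plot.
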(event `HideUI`
  (`SceneComponent.SetVisibility` (`self.BuildUI`) false false)
  (`SceneComponent.SetVisibility` (`self.SellUI`) false false)
  (`SceneComponent.SetVisibility` (`self.UpgradeUI`) false false))

(event `self.ReceiveBeginPlay`
  (bind _upgradeui (`self.UpgradeUI`))
  (bind _buildui (`self.BuildUI`))
  (bind _sellui (`self.SellUI`))
  (`SceneComponent.SetVisibility` _buildui false false)
  (bind _asw_tower_menu (cast `/Game/Blueprints/UI/W_TowerMenu` (`WidgetComponent.GetWidget` _buildui)))
  (bind _returnvalue (`GameplayStatics.GetActorOfClass` "/Game/Blueprints/Gameplay/BP_GameManager.BP_GameManager_C"))
  (set `self.GM_Ref` _returnvalue)
  (`/Game/Blueprints/UI/W_TowerMenu.InitMenu` _asw_tower_menu self (`self.GM_Ref`))
  (`SceneComponent.SetVisibility` _sellui false false)
  (bind _asw_sell_menu (cast `/Game/Blueprints/UI/W_SellMenu` (`WidgetComponent.GetWidget` _sellui)))
  (`/Game/Blueprints/UI/W_SellMenu.InitMenu` _asw_sell_menu self)
  (`SceneComponent.SetVisibility` _upgradeui false false)
  (bind _asw_upgrade_menu (cast `/Game/Blueprints/UI/W_UpgradeMenu` (`WidgetComponent.GetWidget` _upgradeui)))
  (set `self.As W Upgrade Menu` _asw_upgrade_menu)
  (`/Game/Blueprints/UI/W_UpgradeMenu.InitMenuUpgrade` _asw_upgrade_menu self))

(event `HideUpgradeUI`
  ;[1 1 1] this doesn't really fix the issue
  (`ActorComponent.SetActive` (`self.UpgradeUI`) false false :!label _label))

(event `/Game/Blueprints/BPI_Interact.Interact`
  (params (PlayerRef :type "/Game/Blueprints/Player/BP_PlayerPawn Object Reference"))
  (set `self.Player Ref` PlayerRef)
  ;[1 1 1] Close all open Build/Sell UI Widgets
  (bind _outactors (`GameplayStatics.GetAllActorsOfClass` "BP_BuildingPlot_C"))
  (for _array_element _outactors
    (`SceneComponent.SetVisibility` (`/Game/Blueprints/BP_BuildingPlot.BuildUI` _array_element) false false)
    (`SceneComponent.SetVisibility` (`/Game/Blueprints/BP_BuildingPlot.SellUI` _array_element) false false))
  (if (`/Game/Blueprints/Gameplay/BP_GameManager.GameEnded` (`self.GM_Ref`))
    _
    (elif (`self.IsOccupied`)
      (`SceneComponent.SetVisibility` (`self.SellUI`) true false)
      (if (== (`/Game/Jake-Towers/BP_TowersMain.TowerLevel` (`self.CurrentTower`)) 3)
        (goto _label)
        (else
          (`SceneComponent.SetVisibility` (`self.UpgradeUI`) true false)))
      (else
        (`SceneComponent.SetVisibility` (`self.BuildUI`) true false)))))

(event `SpawnTower`
  (params (TowerType :type "/Game/Jake-Towers/E_TowerTypes Enum" :default "NewEnumerator0"))
  (set `self.Tower Type` TowerType)
  (if (not (`self.IsOccupied`))
    (`PrimitiveComponent.SetMaterial` (`self.BaseMesh`) 0 "/Game/Icons/Cursor_Mat.Cursor_Mat")
    (bind _returnvalue (`|SpawnActorFromClass` "/Game/Jake-Towers/BP_TowersMain.BP_TowersMain_C" (`SceneComponent.K2_GetComponentToWorld` (`self.TowerSpawn`)) "Undefined" "OverrideRootScale" null null))
    (`/Game/Jake-Towers/BP_TowersMain.Init_Tower` _returnvalue TowerType (`self.GM_Ref`) self)
    (set `self.CurrentTower` _returnvalue)
    (`/Game/Blueprints/UI/W_UpgradeMenu.UpdateTowerText` (`self.As W Upgrade Menu`))
    (set `self.IsOccupied` true)
    (`SceneComponent.SetVisibility` (`self.BuildUI`) false false)))

(event `SellTower`
  (bind _currenttower (`self.CurrentTower`))
  (`/Engine/EditorBlueprintResources/StandardMacros.IsValid` _currenttower
    (:`Is Valid`
      (`/Game/Jake-Towers/BP_TowersMain.ExplodeTimer` _currenttower)
      (set `self.IsOccupied` false)
      (`self.HideUI`)
      (`PrimitiveComponent.SetMaterial` (`self.BaseMesh`) 0 "/Engine/EngineMaterials/WorldGridMaterial.WorldGridMaterial")
      (`GameplayStatics.PlaySound2D` "/Game/Audio/SFX/Grenade_Bomb_-_Small_Dull_Explosion_Burst_-_01_____002567_.Grenade_Bomb_-_Small_Dull_Explosion_Burst_-_01_____002567_" 0.2 1.0 0.0 null null false))))

(event `TowerReachedMaxLevel`
  ;[1 1 1] Disable button - Tower is max level
  (`ActorComponent.SetActive` (`self.UpgradeUI`) false false))

(fn `UserConstructionScript`)