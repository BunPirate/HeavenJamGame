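; BP_Currency tracks the player's Souls currency and keeps the HUD currency widget in sync.
; Init stores a game mode reference and pushes the starting count to the UI through its HUD widget.
; AddSouls adds the stored SoulsToAdd amount, while RemoveSouls subtracts a passed amount clamped at zero, and both refresh the UI afterward.
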(event `Init_Currency`
  (params (GM_Ref :type "/Game/Blueprints/Gameplay/BP_GameManager Object Reference"))
  ;[1 1 1] Init
  (bind _output_get (set `self.GM Ref` GM_Ref))
  (`/Game/Jake-Towers/W_Currency.UpdateSoulsUI` (`/Game/Blueprints/UI/HUD_Main.W_Currency` (`/Game/Blueprints/Gameplay/BP_GameManager.HUD_UI_Ref` _output_get)) (`self.CurrentSouls`)))

(event `AddSouls`
  ;[1 1 1] Add Souls + Update Souls UI-- Don't remove update souls bits XD
  (bind _output_get (set `self.CurrentSouls` (+ (`self.SoulsToAdd`) (`self.CurrentSouls`))))
  (`/Game/Jake-Towers/W_Currency.UpdateSoulsUI` (`/Game/Blueprints/UI/HUD_Main.W_Currency` (`/Game/Blueprints/Gameplay/BP_GameManager.HUD_UI_Ref` (`self.GM Ref`))) _output_get))

(event `RemoveSouls`
  (params (SoulsToTake :type Integer))
  (bind _returnvalue (- (`self.CurrentSouls`) (`self.SoulsToRemove`)))
  ;[1 1 1] Remove Souls + Update Souls UI
  (set `self.SoulsToRemove` SoulsToTake)
  (if (< _returnvalue 0)
    (set `self.CurrentSouls` 0)
    (else
      (set `self.CurrentSouls` _returnvalue)))
  (`/Game/Jake-Towers/W_Currency.UpdateSoulsUI` (`/Game/Blueprints/UI/HUD_Main.W_Currency` (`/Game/Blueprints/Gameplay/BP_GameManager.HUD_UI_Ref` (`self.GM Ref`))) (`self.CurrentSouls`)))