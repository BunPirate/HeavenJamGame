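; Base projectile for tower bullets that damages enemies it touches.
; BeginPlay sets the projectile movement speed from BulletSpeed, caps it, and destroys the actor after a fixed lifetime.
; Sphere overlaps are matched against a loop over all BP_EnemyBase actors; a match receives DoDamageMessage with a fixed team and Damage, then the projectile destroys itself.
; GetEnemy is an empty stub.
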(event `self.Sphere.OnComponentBeginOverlap`
  (params (OverlappedComponent :type "PrimitiveComponent Object Reference") (OtherActor :type "Actor Object Reference") (OtherComp :type "PrimitiveComponent Object Reference") (OtherBodyIndex :type Integer) (bFromSweep :type Boolean) (SweepResult :type "HitResult Structure (by ref)"))
  (bind _outactors (`GameplayStatics.GetAllActorsOfClass` "/Game/Blueprints/Enemies/BP_EnemyBase.BP_EnemyBase_C"))
  (for _array_element _outactors
    (if (== OtherActor _array_element)
      (message `/Game/Blueprints/Enemies/BPI_Damage.DoDamage` _array_element "NewEnumerator0" (`self.Damage`))
      (`self.K2_DestroyActor`))))

(event `self.ReceiveBeginPlay`
  (bind _projectilemovement (`self.ProjectileMovement`))
  (set `ProjectileMovementComponent.InitialSpeed` (`self.BulletSpeed`) _projectilemovement)
  (set `ProjectileMovementComponent.MaxSpeed` 3000.0 _projectilemovement)
  (`KismetSystemLibrary.Delay` 6.0)
  (`self.K2_DestroyActor`))

(fn `GetEnemy`
  (returns (EnemyBase :type "/Game/Blueprints/Enemies/BP_EnemyBase Object Reference"))
  (return null))

(fn `UserConstructionScript`)