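; BP_Bomb is a bomb projectile Blueprint for towers that leaves a Niagara effect when it is destroyed.
; Tick caches the actor's location every frame after running the parent logic.
; The Destroyed event spawns NS_Bomb at that cached location at reduced scale.
; BeginPlay only calls the parent, and no movement or damage logic is defined in this graph.
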(event `self.ReceiveBeginPlay`
  (`parent.ReceiveBeginPlay`))

(event `self.ReceiveTick`
  (params (DeltaSeconds :type "Float (single-precision)"))
  (`parent.ReceiveTick` DeltaSeconds)
  (set `self.Location` (`self.K2_GetActorLocation`)))

(event `self.ReceiveDestroyed`
  (`NiagaraFunctionLibrary.SpawnSystemAtLocation` "/Game/Particles/NS_Bomb.NS_Bomb" (`self.Location`) (struct) (0.5 0.5 0.5)))

(fn `UserConstructionScript`
  (`parent.UserConstructionScript`))