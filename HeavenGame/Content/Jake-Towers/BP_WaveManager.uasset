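; Wave manager for a tower defense game that picks a setup by level name; only Level 1 is implemented, the others are print stubs.
; A looping timer spawns fast or tanky enemies at the spline start, with later mixes split by remaining count rather than randomly.
; After a delay, NextWave advances the wave and UI, but returns false upon reaching the maximum.
; LevelBeat, called beyond that maximum, polls for zero enemies to show completion UI.
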(event `Init_WaveManager`
  (params (UI_Ref :type "/Game/Blueprints/UI/HUD_Main Object Reference") (GM_Ref :type "/Game/Blueprints/Gameplay/BP_GameManager Object Reference"))
  ;[1 1 1] Init Chain
  (set `self.UI Ref` UI_Ref)
  (set `self.GM Ref` GM_Ref)
  (bind _returnvalue (`GameplayStatics.GetCurrentLevelName` true))
  (`self.SwitchToSelectedLevel` _returnvalue))

(event `WaveComplete`
  (bind _currentwave (`self.CurrentWave`))
  ;[1 1 1] Level 1 Setup
  ;;[1 1 1] Wave Complete - Trigger Next
  (bind _success (`self.NextWave`))
  (if _success
    (`KismetSystemLibrary.PrintString` (`KismetStringLibrary.Concat_StrStr` "Wave Num: " (`KismetStringLibrary.Conv_IntToString` _currentwave)) true true (struct :`R` 1.0 :`G` 0.056409 :`A` 1.0) 8.0)
    (switch `int` _currentwave :!label _label
      (:`1`
        (set `self.WaveSize` 4))
      (:`2`
        (set `self.WaveSize` 6))
      (:`3`
        (set `self.WaveSize` 8))
      (:`4`
        (set `self.WaveSize` 10))
      (:`5`
        (set `self.WaveSize` 12)))
    (bind _returnvalue (`KismetSystemLibrary.K2_SetTimer` null "SpawnTroops" 5.0 true))
    (set `self.Wave1Timer` _returnvalue)))

(event `Level1`
  ;[1 1 1] Level 1 Setup
  (if (`self.Active`)
    (set `self.Active` false)
    (set `self.MaxNumWaves` 5)
    (set `self.TotalTroopCount` 40)
    (goto _label)))

(event `SpawnTroops`
  ;[1 1 1] Spawn Enemies
  (bind _result (`/Engine/EditorBlueprintResources/StandardMacros.DecrementInt` (`self.WaveSize`))
    (:`  `
      (set `self.WaveSize` _result)
      (if (>= (`self.WaveSize`) 0)
        (switch `int` (`self.CurrentWave`)
          (:`1`
            (`self.SpawnEnemyTypeFaste`))
          (:`2`
            (`self.SpawnEnemyTypeTanky`))
          (:`3`
            (`self.SpawnRandomEnemyL1-W3`))
          (:`4`
            (`self.SpawnRandomEnemyL1-W4`))
          (:`5`
            (`self.SpawnRandomEnemyL1-W5`)))
        (else
          (`KismetSystemLibrary.PrintString` "Wave Complete Trigger Next" true true (struct :`R` 1.0 :`B` 0.021375 :`A` 1.0) 8.0)
          (`KismetSystemLibrary.K2_ClearAndInvalidateTimerHandle` (`self.Wave1Timer`))
          (`KismetSystemLibrary.Delay` (`self.DelayBetweenWaves`))
          (`self.WaveComplete`))))))

(event `Level2`
  (`KismetSystemLibrary.PrintString` "Level 2" true true (struct :`R` 1.0 :`B` 0.039438 :`A` 1.0) 8.0))

(event `Level3`
  (`KismetSystemLibrary.PrintString` "Level 3" true true (struct :`R` 1.0 :`B` 0.039438 :`A` 1.0) 8.0))

(event `LevelBeat`
  ;[1 1 1] Level Beat Show UI
  (bind _returnvalue (`KismetSystemLibrary.K2_SetTimerDelegate` (delegate `Check`) 1.0 true))
  (set `self.CheckForWin` _returnvalue))

(event `Check`
  ;[1 1 1] Level Beat Show UI
  (`KismetSystemLibrary.PrintString` "FINISHHHH")
  (bind _outactors (`GameplayStatics.GetAllActorsOfClass` "/Game/Blueprints/Enemies/BP_EnemyBase.BP_EnemyBase_C"))
  (if (<= (`KismetArrayLibrary.Array_Length` _outactors) 0)
    (`/Game/Blueprints/UI/W_LevelComplete.GameCompleteUI` (`/Game/Blueprints/UI/HUD_Main.W_LevelComplete` (`self.UI Ref`)))
    (set `/Game/Blueprints/Gameplay/BP_GameManager.GameEnded` false (`self.GM Ref`))
    (`KismetSystemLibrary.K2_ClearAndInvalidateTimerHandle` (`self.CheckForWin`))))

(fn `NextWave`
  (returns (Success :type Boolean))
  (bind _currentwave (`self.CurrentWave`))
  (bind _returnvalue (< _currentwave (`self.MaxNumWaves`)))
  (if _returnvalue
    (bind _result (`/Engine/EditorBlueprintResources/StandardMacros.IncrementInt` _currentwave)
      (:`  `
        (bind _output_get (set `self.CurrentWave` _result))
        (`/Game/Blueprints/UI/W_WaveUI.UpdateWaveUI` (`/Game/Blueprints/UI/HUD_Main.W_WaveUI_Current` (`self.UI Ref`)) _output_get)
        (return _returnvalue)))
    (else
      (`KismetSystemLibrary.PrintString` "Level Complete - Add an event dispatcher")
      (`self.LevelBeat`))))

(fn `SpawnEnemyTypeFaste`
  (bind _gm_ref (`self.GM Ref`))
  (bind _returnvalue (`|SpawnActorFromClass` "/Game/Blueprints/Enemies/BP_FastEnemy.BP_FastEnemy_C" (`KismetMathLibrary.MakeTransform` (`SplineComponent.GetLocationAtSplinePoint` (`/Game/Blueprints/Gameplay/BP_GameManager.Spline` _gm_ref) 0 "World")) "Undefined" "OverrideRootScale" null null))
  (`/Game/Blueprints/Enemies/BP_EnemyBase.InitEnemy` _returnvalue _gm_ref))

(fn `SpawnEnemyTypeTanky`
  (bind _gm_ref (`self.GM Ref`))
  (bind _returnvalue (`|SpawnActorFromClass` "/Game/Blueprints/Enemies/BP_TankyEnemy.BP_TankyEnemy_C" (`KismetMathLibrary.MakeTransform` (`SplineComponent.GetLocationAtSplinePoint` (`/Game/Blueprints/Gameplay/BP_GameManager.Spline` _gm_ref) 0 "World")) "Undefined" "OverrideRootScale" null null))
  (`/Game/Blueprints/Enemies/BP_EnemyBase.InitEnemy` _returnvalue _gm_ref))

(fn `SpawnRandomEnemyL1-W3`
  (bind _gm_ref (`self.GM Ref`))
  (bind _gm_ref_2 (`self.GM Ref`))
  (if (<= (`self.WaveSize`) 5)
    (bind _returnvalue (`|SpawnActorFromClass` "/Game/Blueprints/Enemies/BP_FastEnemy.BP_FastEnemy_C" (`KismetMathLibrary.MakeTransform` (`SplineComponent.GetLocationAtSplinePoint` (`/Game/Blueprints/Gameplay/BP_GameManager.Spline` _gm_ref_2) 0 "World")) "Undefined" "OverrideRootScale" null null))
    (`/Game/Blueprints/Enemies/BP_EnemyBase.InitEnemy` _returnvalue _gm_ref_2)
    (else
      (bind _returnvalue_2 (`|SpawnActorFromClass` "/Game/Blueprints/Enemies/BP_TankyEnemy.BP_TankyEnemy_C" (`KismetMathLibrary.MakeTransform` (`SplineComponent.GetLocationAtSplinePoint` (`/Game/Blueprints/Gameplay/BP_GameManager.Spline` _gm_ref) 0 "World")) "Undefined" "OverrideRootScale" null null))
      (`/Game/Blueprints/Enemies/BP_EnemyBase.InitEnemy` _returnvalue_2 _gm_ref))))

(fn `SpawnRandomEnemyL1-W4`
  (bind _gm_ref (`self.GM Ref`))
  (bind _gm_ref_2 (`self.GM Ref`))
  (if (<= (`self.WaveSize`) 5)
    (bind _returnvalue (`|SpawnActorFromClass` "/Game/Blueprints/Enemies/BP_FastEnemy.BP_FastEnemy_C" (`KismetMathLibrary.MakeTransform` (`SplineComponent.GetLocationAtSplinePoint` (`/Game/Blueprints/Gameplay/BP_GameManager.Spline` _gm_ref_2) 0 "World")) "Undefined" "OverrideRootScale" null null))
    (`/Game/Blueprints/Enemies/BP_EnemyBase.InitEnemy` _returnvalue _gm_ref_2)
    (else
      (bind _returnvalue_2 (`|SpawnActorFromClass` "/Game/Blueprints/Enemies/BP_TankyEnemy.BP_TankyEnemy_C" (`KismetMathLibrary.MakeTransform` (`SplineComponent.GetLocationAtSplinePoint` (`/Game/Blueprints/Gameplay/BP_GameManager.Spline` _gm_ref) 0 "World")) "Undefined" "OverrideRootScale" null null))
      (`/Game/Blueprints/Enemies/BP_EnemyBase.InitEnemy` _returnvalue_2 _gm_ref))))

(fn `SpawnRandomEnemyL1-W5`
  (bind _gm_ref (`self.GM Ref`))
  (bind _gm_ref_2 (`self.GM Ref`))
  (if (>= (`self.WaveSize`) 5)
    (bind _returnvalue (`|SpawnActorFromClass` "/Game/Blueprints/Enemies/BP_FastEnemy.BP_FastEnemy_C" (`KismetMathLibrary.MakeTransform` (`SplineComponent.GetLocationAtSplinePoint` (`/Game/Blueprints/Gameplay/BP_GameManager.Spline` _gm_ref_2) 0 "World")) "Undefined" "OverrideRootScale" null null))
    (`/Game/Blueprints/Enemies/BP_EnemyBase.InitEnemy` _returnvalue _gm_ref_2)
    (else
      (bind _returnvalue_2 (`|SpawnActorFromClass` "/Game/Blueprints/Enemies/BP_TankyEnemy.BP_TankyEnemy_C" (`KismetMathLibrary.MakeTransform` (`SplineComponent.GetLocationAtSplinePoint` (`/Game/Blueprints/Gameplay/BP_GameManager.Spline` _gm_ref) 0 "World")) "Undefined" "OverrideRootScale" null null))
      (`/Game/Blueprints/Enemies/BP_EnemyBase.InitEnemy` _returnvalue_2 _gm_ref))))

(fn `SwitchToSelectedLevel`
  (params (LevelName :type String))
  ;[1 1 1] Switch to selected Level
  (switch `string` LevelName
    (:`L_TestMap`
      (`self.Level1`))
    (:`Level2`
      (`self.Level2`))
    (:`Level3`
      (`self.Level3`))))