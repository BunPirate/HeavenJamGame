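; Tower-defense tower actor for four types, with material, bullet class and per-level stats set through Init_Tower.
; AttackRadius overlaps track tagged enemies; a looping search picks the one furthest along its spline, and a fire-rate timer spawns bullets aimed at it.
; Upgrades spend souls from the GameMode reference's currency and reapply stats.
; A lifetime timer explodes the tower, frees its plot and refunds roughly half its cost in souls.
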(event `Init_Tower`
  (params (TowerType :type "/Game/Jake-Towers/E_TowerTypes Enum" :default "NewEnumerator0") (GM_Ref :type "/Game/Blueprints/Gameplay/BP_GameManager Object Reference") (PlotRef :type "/Game/Blueprints/BP_BuildingPlot Object Reference"))
  ;[0.7192 1 0.4582] Init Chain For Refs + Setup
  (set `self.Plot Ref` PlotRef)
  (set `self.GM_Ref` GM_Ref)
  (bind _output_get (set `self.TowerType_NEW` TowerType))
  (`self.SetTowerType` _output_get)
  (`self.SetupTowerStats`)
  (`self.Tower Health Debug`)
  (bind _returnvalue (`KismetSystemLibrary.K2_SetTimer` null "Searching" 0.25 true))
  (set `self.SearchingTimer` _returnvalue)
  (bind _returnvalue_2 (`KismetSystemLibrary.K2_SetTimerDelegate` (delegate `TowerLifetime`) 1.0 true))
  (set `self.TowerLifeTimeTimer` _returnvalue_2))

(event `UpgradeTower`
  (params (TowerType :type "/Game/Jake-Towers/E_TowerTypes Enum" :default "NewEnumerator0"))
  ;[1 1 1] Upgrade Towers
  (`KismetSystemLibrary.PrintString` "Tower Upgraded" true true (struct :`R` 1.0 :`G` 0.121925 :`A` 1.0) 8.0)
  (bind _success (`self.UpgradeTowerLevel` TowerType))
  (if _success
    (`self.SetupTowerStats`)))

(event `TowerLifetime`
  ;[1 1 1] Towers auto-destruct after set duration
  (if (not (`/Game/Blueprints/Gameplay/BP_GameManager.GameEnded` (`self.GM_Ref`)))
    (bind _result (`/Engine/EditorBlueprintResources/StandardMacros.IncrementInt` (`self.Time`))
      (:`  `
        (bind _output_get (set `self.Time` _result))
        (`KismetSystemLibrary.PrintString` (`KismetStringLibrary.Conv_IntToString` _output_get))
        (if (> _output_get (`self.SelfDestructTime`))
          (`self.ExplodeTimer`))))))

(event `SauronEyeTower`
  ;[0.503 1 0.5281] Initilise Each Tower Type Setting their bullet types + Meshes/Materials
  (`PrimitiveComponent.SetMaterial` (`self.TowerMesh`) 0 "/Game/Jake-Towers/Temp_Materials/M_TowersRed.M_TowersRed")
  (set `self.BulletType` "/Game/Jake-Towers/Bullets/BP_S_Bullet.BP_S_Bullet_C"))

(event `BarracksTower`
  ;[0.503 1 0.5281] Initilise Each Tower Type Setting their bullet types + Meshes/Materials
  (`PrimitiveComponent.SetMaterial` (`self.TowerMesh`) 0 "/Game/Jake-Towers/Temp_Materials/M_TowersOrange.M_TowersOrange")
  (set `self.BulletType` "/Game/Jake-Towers/Bullets/BP_B_Bullet.BP_B_Bullet_C"))

(event `LavaBomberTower`
  ;[0.503 1 0.5281] Initilise Each Tower Type Setting their bullet types + Meshes/Materials
  (`PrimitiveComponent.SetMaterial` (`self.TowerMesh`) 0 "/Game/Jake-Towers/Temp_Materials/M_TowersYellow.M_TowersYellow")
  (set `self.BulletType` "/Game/Jake-Towers/Bullets/BP_L_Bomb.BP_L_Bomb_C"))

(event `ImpBomber`
  ;[0.503 1 0.5281] Initilise Each Tower Type Setting their bullet types + Meshes/Materials
  (`PrimitiveComponent.SetMaterial` (`self.TowerMesh`) 0 "/Game/Jake-Towers/Temp_Materials/M_TowersBlue.M_TowersBlue")
  (set `self.BulletType` "/Game/Jake-Towers/Bullets/BP_B_Bullet.BP_B_Bullet_C"))

(event `self.AttackRadius.OnComponentBeginOverlap`
  (params (OverlappedComponent :type "PrimitiveComponent Object Reference") (OtherActor :type "Actor Object Reference") (OtherComp :type "PrimitiveComponent Object Reference") (OtherBodyIndex :type Integer) (bFromSweep :type Boolean) (SweepResult :type "HitResult Structure (by ref)"))
  (bind _activetargets (`self.ActiveTargets`))
  ;[0.2956 1 0.7237] Tower Attack Radius Triggers
  (if (`self.TowerAwake`)
    (if (`KismetArrayLibrary.Array_Contains` _activetargets OtherActor)
      _
      (elif (and (`KismetSystemLibrary.IsValid` OtherActor) (`self.ActorHasTag` OtherActor "Enemy"))
        (`KismetArrayLibrary.Array_Add` _activetargets OtherActor)
        (set `self.SearchForTarget` true)))))

(event `self.AttackRadius.OnComponentEndOverlap`
  (params (OverlappedComponent :type "PrimitiveComponent Object Reference") (OtherActor :type "Actor Object Reference") (OtherComp :type "PrimitiveComponent Object Reference") (OtherBodyIndex :type Integer))
  (bind _activetargets (`self.ActiveTargets`))
  ;[0.2956 1 0.7237] Tower Attack Radius Triggers
  (if (`self.TowerAwake`)
    (if (`KismetArrayLibrary.Array_Contains` _activetargets OtherActor)
      (if (== OtherActor (`self.FoundTarget`))
        (set `self.TargetSelected` false)
        (`KismetArrayLibrary.Array_RemoveItem` _activetargets OtherActor)
        (else
          (`KismetArrayLibrary.Array_RemoveItem` (`self.ActiveTargets`) OtherActor))))))

(event `Searching`
  ;[0.03839 1 0.3633] Check to see if there is a Target Selected - If no target is selected find new one - Start Shooting
  (if (`self.SearchForTarget`)
    (if (not (`self.TargetSelected`))
      (`self.FindClosestTarget`))))

(event `ShootTarget`
  ;[0.3882 1 0.5623] Set looping timer - Rotate towards target - Fire at target
  (bind _returnvalue (`KismetSystemLibrary.K2_SetTimerDelegate` (delegate `SpawnBullets`) (`self.FireRate`) true))
  (set `self.ShootTimer` _returnvalue))

(event `SpawnBullets`
  (bind _returnvalue (`SceneComponent.K2_GetComponentLocation` (`self.FirePoint`)))
  ;[0.3882 1 0.5623] Set looping timer - Rotate towards target - Fire at target
  (if (and (`KismetSystemLibrary.IsValid` (`self.FoundTarget`)) (`KismetArrayLibrary.Array_Contains` (`self.ActiveTargets`) (`self.FoundTarget`)))
    ;;[0.3645 1 0.9901] Rotate FirePoint to target look at rotation (Rotate to target location)
    (`SceneComponent.K2_SetWorldRotation` (`self.FirePoint`) (`KismetMathLibrary.FindLookAtRotation` (`SceneComponent.K2_GetComponentLocation` (`self.FirePoint`)) (`self.K2_GetActorLocation` (`self.FoundTarget`))) false false)
    ;;[0.4479 1 1] Fire Bullets
    (`|SpawnActorFromClass` (`self.BulletType`) (`KismetMathLibrary.MakeTransform` _returnvalue (`KismetMathLibrary.FindLookAtRotation` _returnvalue (`self.K2_GetActorLocation` (`self.FoundTarget`)))) "Undefined" "OverrideRootScale" null null)
    (else
      (`KismetSystemLibrary.PrintString` "No Target")
      (`KismetArrayLibrary.Array_RemoveItem` (`self.ActiveTargets`) (`self.FoundTarget`))
      (set `self.SearchForTarget` true)
      (set `self.TargetSelected` false)
      (`KismetSystemLibrary.K2_ClearAndInvalidateTimerHandle` (`self.ShootTimer`))
      (`self.Searching`))))

(fn `ExplodeTimer`
  (bind _plot_ref (`self.Plot Ref`))
  ;[1 1 1] Add some sounds/explosion maybe add some souls
  (`KismetSystemLibrary.PrintString` "Tower Goes Boom" true true (struct :`R` 1.0 :`G` 0.008451 :`A` 1.0) 8.0)
  (`self.CalculateSoulsToAdd`
    (:`NewParam2`
      ;;[1 1 1] Needs to be done otherwise sell menu remains
      (set `/Game/Blueprints/BP_BuildingPlot.IsOccupied` false _plot_ref)
      (`PrimitiveComponent.SetMaterial` (`/Game/Blueprints/BP_BuildingPlot.BaseMesh` _plot_ref) 0 "/Engine/EngineMaterials/WorldGridMaterial.WorldGridMaterial")
      (`/Game/Jake-Towers/BP_Currency.AddSouls` (`/Game/Blueprints/Gameplay/BP_GameManager.BP_Currency` (`self.GM_Ref`)) (`self.SoulsToAdd`))
      (`NiagaraFunctionLibrary.SpawnSystemAtLocation` "/Game/Jake-Towers/Particles/P_Explode.P_Explode" (- (`SceneComponent.K2_GetComponentLocation` (`self.FirePoint`)) (0.0 0.0 -80.0)) (struct) (2.0 2.0 2.0))
      (`self.K2_DestroyActor`))))

(fn `FindClosestTarget`
  ;[0.5884 1 0.3767] Find Closest Target - Count Total Num of Targets
  (if (`self.SearchForTarget`)
    (set `self.SearchForTarget` false)
    (for _array_element (`self.ActiveTargets`)
      (if (`KismetSystemLibrary.IsValid` _array_element)
        (bind _enemybase (message `/Game/Blueprints/Enemies/BPI_Damage.GetEnemy` _array_element))
        (bind _progressalongspline (`/Game/Blueprints/Enemies/BP_EnemyBase.ProgressAlongSpline` _enemybase))
        (if (>= _progressalongspline (`self.ClosestEnemy`))
          (set `self.ClosestEnemy` _progressalongspline)
          (if (`KismetSystemLibrary.IsValid` _enemybase)
            (set `self.TargetSelected` true)
            (set `self.FoundTarget` _array_element)))))
    (`KismetSystemLibrary.PrintString` "Target SET" true true (struct :`R` 1.0 :`B` 0.018539 :`A` 1.0) 8.0)
    (`self.ShootTarget`)))

(fn `GetEnemy`
  (returns (EnemyBase :type "/Game/Blueprints/Enemies/BP_EnemyBase Object Reference"))
  (return null))

(fn `SetTowerType`
  (params (TowerType :type "/Game/Jake-Towers/E_TowerTypes Enum" :default "NewEnumerator0"))
  ;[0 1 0.2182] Switch on Tower Type - Just to show colour/difference
  (switch `/Game/Jake-Towers/E_TowerTypes` TowerType
    (:`NewEnumerator0`
      (`self.SauronEyeTower`))
    (:`NewEnumerator1`
      (`self.BarracksTower`))
    (:`NewEnumerator2`
      (`self.LavaBomberTower`))
    (:`NewEnumerator3`
      (`self.ImpBomber`))))

(fn `SetupTowerStats`
  ;[1 0.1175 0.2273] Set Stats for Towers will collapse all the sets - Damage is done in bullets not here................
  (switch `/Game/Jake-Towers/E_TowerTypes` (`self.TowerType_NEW`)
    (:`NewEnumerator0`
      (switch `int` (`self.TowerLevel`)
        (:`1`
          (set `self.MaxHealth` 100.0)
          (set `self.Health` 100.0)
          (set `self.DamageMin` 5)
          (set `self.DamageMax` 10)
          (set `self.CriticalHitChance` 5)
          (set `self.FireRate` 0.3)
          (bind _output_get (set `self.AttackRange` 800.0))
          (`SphereComponent.SetSphereRadius` (`self.AttackRadius`) _output_get true)
          (`self.Tower Health Debug`))
        (:`2`
          (set `self.MaxHealth` 125.0)
          (set `self.Health` 125.0)
          (set `self.DamageMin` 6)
          (set `self.DamageMax` 12)
          (set `self.CriticalHitChance` 8)
          (set `self.FireRate` 0.28)
          (bind _output_get_2 (set `self.AttackRange` 850.0))
          (`SphereComponent.SetSphereRadius` (`self.AttackRadius`) _output_get_2 true)
          (`self.Tower Health Debug`))
        (:`3`
          (set `self.MaxHealth` 150.0)
          (set `self.Health` 150.0)
          (set `self.DamageMin` 8)
          (set `self.DamageMax` 14)
          (set `self.CriticalHitChance` 10)
          (set `self.FireRate` 0.25)
          (bind _output_get_3 (set `self.AttackRange` 900.0))
          (`SphereComponent.SetSphereRadius` (`self.AttackRadius`) _output_get_3 true)
          (`self.Tower Health Debug`))))
    (:`NewEnumerator1`
      (switch `int` (`self.TowerLevel`)
        (:`1`
          (set `self.MaxHealth` 50.0)
          (set `self.Health` 50.0)
          (set `self.DamageMin` 5)
          (set `self.DamageMax` 10)
          (set `self.CriticalHitChance` 5)
          (set `self.FireRate` 0.2)
          (bind _output_get_4 (set `self.AttackRange` 600.0))
          (`SphereComponent.SetSphereRadius` (`self.AttackRadius`) _output_get_4 true)
          (`self.Tower Health Debug`))
        (:`2`
          (set `self.MaxHealth` 75.0)
          (set `self.Health` 75.0)
          (set `self.DamageMin` 6)
          (set `self.DamageMax` 10)
          (set `self.CriticalHitChance` 5)
          (set `self.FireRate` 0.18)
          (bind _output_get_5 (set `self.AttackRange` 650.0))
          (`SphereComponent.SetSphereRadius` (`self.AttackRadius`) _output_get_5 true)
          (`self.Tower Health Debug`))
        (:`3`
          (set `self.MaxHealth` 100.0)
          (set `self.Health` 100.0)
          (set `self.DamageMin` 5)
          (set `self.DamageMax` 10)
          (set `self.CriticalHitChance` 5)
          (set `self.FireRate` 0.16)
          (bind _output_get_6 (set `self.AttackRange` 700.0))
          (`SphereComponent.SetSphereRadius` (`self.AttackRadius`) _output_get_6 true)
          (`self.Tower Health Debug`))))
    (:`NewEnumerator2`
      (switch `int` (`self.TowerLevel`)
        (:`1`
          (set `self.MaxHealth` 250.0)
          (set `self.Health` 250.0)
          (set `self.DamageMin` 5)
          (set `self.DamageMax` 10)
          (set `self.CriticalHitChance` 5)
          (set `self.FireRate` 0.5)
          (bind _output_get_7 (set `self.AttackRange` 1200.0))
          (`SphereComponent.SetSphereRadius` (`self.AttackRadius`) _output_get_7 true)
          (`self.Tower Health Debug`))
        (:`2`
          (set `self.MaxHealth` 275.0)
          (set `self.Health` 275.0)
          (set `self.DamageMin` 5)
          (set `self.DamageMax` 10)
          (set `self.CriticalHitChance` 5)
          (set `self.FireRate` 0.46)
          (bind _output_get_8 (set `self.AttackRange` 1250.0))
          (`SphereComponent.SetSphereRadius` (`self.AttackRadius`) _output_get_8 true)
          (`self.Tower Health Debug`))
        (:`3`
          (set `self.MaxHealth` 250.0)
          (set `self.Health` 250.0)
          (set `self.DamageMin` 5)
          (set `self.DamageMax` 10)
          (set `self.CriticalHitChance` 5)
          (set `self.FireRate` 0.44)
          (bind _output_get_9 (set `self.AttackRange` 1300.0))
          (`SphereComponent.SetSphereRadius` (`self.AttackRadius`) _output_get_9 true)
          (`self.Tower Health Debug`))))
    (:`NewEnumerator3`
      (switch `int` (`self.TowerLevel`)
        (:`1`
          (set `self.MaxHealth` 10.0)
          (set `self.Health` 10.0)
          (set `self.DamageMin` 5)
          (set `self.DamageMax` 10)
          (set `self.CriticalHitChance` 5)
          (set `self.FireRate` 0.18)
          (bind _output_get_10 (set `self.AttackRange` 500.0))
          (`SphereComponent.SetSphereRadius` (`self.AttackRadius`) _output_get_10 true)
          (`self.Tower Health Debug`))
        (:`2`
          (set `self.MaxHealth` 14.0)
          (set `self.Health` 14.0)
          (set `self.DamageMin` 5)
          (set `self.DamageMax` 10)
          (set `self.CriticalHitChance` 5)
          (set `self.FireRate` 0.16)
          (bind _output_get_11 (set `self.AttackRange` 600.0))
          (`SphereComponent.SetSphereRadius` (`self.AttackRadius`) _output_get_11 true)
          (`self.Tower Health Debug`))
        (:`3`
          (set `self.MaxHealth` 16.0)
          (set `self.Health` 16.0)
          (set `self.DamageMin` 5)
          (set `self.DamageMax` 10)
          (set `self.CriticalHitChance` 5)
          (set `self.FireRate` 0.12)
          (bind _output_get_12 (set `self.AttackRange` 700.0))
          (`SphereComponent.SetSphereRadius` (`self.AttackRadius`) _output_get_12 true)
          (`self.Tower Health Debug`))))))

(fn `Tower Health Debug`
  (switch `/Game/Jake-Towers/E_TowerTypes` (`self.TowerType`)
    (:`NewEnumerator0`
      (`self.HealthSetup`))
    (:`NewEnumerator1`
      (`self.HealthSetup`))
    (:`NewEnumerator2`
      (`self.HealthSetup`))
    (:`NewEnumerator3`
      (`self.HealthSetup`))))

(fn `UpgradeTowerLevel`
  (params (Tower :type "/Game/Jake-Towers/E_TowerTypes Enum" :default "NewEnumerator0"))
  (returns (Success :type Boolean))
  (bind ((`SauronLevel2_16_001CCF2F4A82E031605B2B9FC4F23EC8` _sauronlevel2) (`BarracksLevel2_18_83F0388244A49FA1BB75AA9DA18E0BE3` _barrackslevel2) (`LavaBomberLevel2_20_84041DF144E90233EE2E19AAE23073C9` _lavabomberlevel2) (`ImpLevel2_22_D38391C44D1393997B3F07B87EE066A5` _implevel2)) (break `/Game/Jake-Towers/S_TowerUpgradeCosts` (`self.TowerUpgradeCosts`)))
  (bind ((`SauronLevel3_17_8905101D466A57A030932285F693B2C4` _sauronlevel3) (`BarracksLevel3_19_9BCCBBC8475556C0F6BF5A9CF543102A` _barrackslevel3) (`LavaBomberLevel3_21_8EEE269A424F0BC272CA2099CB015680` _lavabomberlevel3) (`ImpLevel3_23_D8CB96CE47CC2702285D7D83A1B0E0F2` _implevel3)) (break `/Game/Jake-Towers/S_TowerUpgradeCosts` (`self.TowerUpgradeCosts`)))
  (bind ((`SauronLevel1_29_62B5E58A4394C3675F024D9899C4F8BE` _sauronlevel1) (`BarracksLevel1_33_6BFA1CB04EDC395EDBEB13B14B7D99AD` _barrackslevel1) (`LavaBomberLevel1_34_280ED3064F03E56B2C2481B02B6B73FB` _lavabomberlevel1) (`ImpLevel1_35_0B0BD4CB43239C8076268C8BB268CCB1` _implevel1)) (break `/Game/Jake-Towers/S_TowerUpgradeCosts` (`self.TowerUpgradeCosts`)))
  (bind _currentsouls (`/Game/Jake-Towers/BP_Currency.CurrentSouls` (`/Game/Blueprints/Gameplay/BP_GameManager.BP_Currency` (`self.GM_Ref`))))
  (bind _currentsouls_2 (`/Game/Jake-Towers/BP_Currency.CurrentSouls` (`/Game/Blueprints/Gameplay/BP_GameManager.BP_Currency` (`self.GM_Ref`))))
  (bind _currentsouls_3 (`/Game/Jake-Towers/BP_Currency.CurrentSouls` (`/Game/Blueprints/Gameplay/BP_GameManager.BP_Currency` (`self.GM_Ref`))))
  (bind _currentsouls_4 (`/Game/Jake-Towers/BP_Currency.CurrentSouls` (`/Game/Blueprints/Gameplay/BP_GameManager.BP_Currency` (`self.GM_Ref`))))
  (bind _currentsouls_5 (`/Game/Jake-Towers/BP_Currency.CurrentSouls` (`/Game/Blueprints/Gameplay/BP_GameManager.BP_Currency` (`self.GM_Ref`))))
  (bind _currentsouls_6 (`/Game/Jake-Towers/BP_Currency.CurrentSouls` (`/Game/Blueprints/Gameplay/BP_GameManager.BP_Currency` (`self.GM_Ref`))))
  (switch `int` (`self.TowerLevel`)
    (:`1`
      ;[1 1 1] Upgrade from Base to Level 1
      (switch `/Game/Jake-Towers/E_TowerTypes` "NewEnumerator0"
        (:`NewEnumerator0`
          (if (<= _sauronlevel1 _currentsouls)
            (`/Game/Jake-Towers/BP_Currency.RemoveSouls` (`/Game/Blueprints/Gameplay/BP_GameManager.BP_Currency` (`self.GM_Ref`)) _sauronlevel1)
            (bind _result (`/Engine/EditorBlueprintResources/StandardMacros.IncrementInt` (`self.TowerLevel`))
              (:`  `
                (set `self.TowerLevel` _result)))
            (else
              (bind _output_get (set `self.UpgradeSuccess` false))
              (return _output_get))))
        (:`NewEnumerator1`
          (if (<= _barrackslevel1 _currentsouls)
            (`/Game/Jake-Towers/BP_Currency.RemoveSouls` (`/Game/Blueprints/Gameplay/BP_GameManager.BP_Currency` (`self.GM_Ref`)) _barrackslevel1)
            (bind _result_2 (`/Engine/EditorBlueprintResources/StandardMacros.IncrementInt` (`self.TowerLevel`))
              (:`  `
                (set `self.TowerLevel` _result_2)))
            (else
              (bind _output_get_2 (set `self.UpgradeSuccess` false))
              (return _output_get_2))))
        (:`NewEnumerator2`
          (if (<= _lavabomberlevel1 _currentsouls_2)
            (`/Game/Jake-Towers/BP_Currency.RemoveSouls` (`/Game/Blueprints/Gameplay/BP_GameManager.BP_Currency` (`self.GM_Ref`)) _lavabomberlevel1)
            (bind _result_3 (`/Engine/EditorBlueprintResources/StandardMacros.IncrementInt` (`self.TowerLevel`))
              (:`  `
                (set `self.TowerLevel` _result_3)))
            (else
              (bind _output_get_3 (set `self.UpgradeSuccess` false))
              (return _output_get_3))))
        (:`NewEnumerator3`
          (if (<= _implevel1 _currentsouls_2)
            (`/Game/Jake-Towers/BP_Currency.RemoveSouls` (`/Game/Blueprints/Gameplay/BP_GameManager.BP_Currency` (`self.GM_Ref`)) _implevel1)
            (bind _result_4 (`/Engine/EditorBlueprintResources/StandardMacros.IncrementInt` (`self.TowerLevel`))
              (:`  `
                (set `self.TowerLevel` _result_4)))
            (else
              (bind _output_get_4 (set `self.UpgradeSuccess` false))
              (return _output_get_4)))))
      (bind _output_get_5 (set `self.UpgradeSuccess` true :!label _label))
      (return _output_get_5))
    (:`2`
      ;[1 1 1] Upgrade from Level 1 to Level 2
      (switch `/Game/Jake-Towers/E_TowerTypes` Tower
        (:`NewEnumerator0`
          (if (<= _sauronlevel2 _currentsouls_4)
            (`/Game/Jake-Towers/BP_Currency.RemoveSouls` (`/Game/Blueprints/Gameplay/BP_GameManager.BP_Currency` (`self.GM_Ref`)) _sauronlevel2)
            (bind _result_5 (`/Engine/EditorBlueprintResources/StandardMacros.IncrementInt` (`self.TowerLevel`))
              (:`  `
                (set `self.TowerLevel` _result_5)
                (goto _label)))
            (else
              (bind _output_get_6 (set `self.UpgradeSuccess` false))
              (return _output_get_6))))
        (:`NewEnumerator1`
          (if (<= _barrackslevel2 _currentsouls_4)
            (`/Game/Jake-Towers/BP_Currency.RemoveSouls` (`/Game/Blueprints/Gameplay/BP_GameManager.BP_Currency` (`self.GM_Ref`)) _barrackslevel2)
            (bind _result_6 (`/Engine/EditorBlueprintResources/StandardMacros.IncrementInt` (`self.TowerLevel`))
              (:`  `
                (set `self.TowerLevel` _result_6)
                (goto _label)))
            (else
              (bind _output_get_7 (set `self.UpgradeSuccess` false))
              (return _output_get_7))))
        (:`NewEnumerator2`
          (if (<= _lavabomberlevel2 _currentsouls_6)
            (`/Game/Jake-Towers/BP_Currency.RemoveSouls` (`/Game/Blueprints/Gameplay/BP_GameManager.BP_Currency` (`self.GM_Ref`)) _lavabomberlevel2)
            (bind _result_7 (`/Engine/EditorBlueprintResources/StandardMacros.IncrementInt` (`self.TowerLevel`))
              (:`  `
                (set `self.TowerLevel` _result_7)
                (goto _label)))
            (else
              (bind _output_get_8 (set `self.UpgradeSuccess` false))
              (return _output_get_8))))
        (:`NewEnumerator3`
          (if (<= _implevel2 _currentsouls_6)
            (`/Game/Jake-Towers/BP_Currency.RemoveSouls` (`/Game/Blueprints/Gameplay/BP_GameManager.BP_Currency` (`self.GM_Ref`)) _implevel2)
            (bind _result_8 (`/Engine/EditorBlueprintResources/StandardMacros.IncrementInt` (`self.TowerLevel`))
              (:`  `
                (set `self.TowerLevel` _result_8)
                (goto _label)))
            (else
              (bind _output_get_9 (set `self.UpgradeSuccess` false))
              (return _output_get_9))))))
    (:`3`
      ;[1 1 1] Level 2 to Level 3
      (switch `/Game/Jake-Towers/E_TowerTypes` "NewEnumerator0"
        (:`NewEnumerator0`
          (if (<= _sauronlevel3 _currentsouls_3)
            (`/Game/Jake-Towers/BP_Currency.RemoveSouls` (`/Game/Blueprints/Gameplay/BP_GameManager.BP_Currency` (`self.GM_Ref`)) _sauronlevel3)
            (bind _result_9 (`/Engine/EditorBlueprintResources/StandardMacros.IncrementInt` (`self.TowerLevel`))
              (:`  `
                (set `self.TowerLevel` _result_9)
                (goto _label)))
            (else
              (bind _output_get_10 (set `self.UpgradeSuccess` false))
              (return _output_get_10))))
        (:`NewEnumerator1`
          (if (<= _barrackslevel3 _currentsouls_3)
            (`/Game/Jake-Towers/BP_Currency.RemoveSouls` (`/Game/Blueprints/Gameplay/BP_GameManager.BP_Currency` (`self.GM_Ref`)) _barrackslevel3)
            (bind _result_10 (`/Engine/EditorBlueprintResources/StandardMacros.IncrementInt` (`self.TowerLevel`))
              (:`  `
                (set `self.TowerLevel` _result_10)
                (goto _label)))
            (else
              (bind _output_get_11 (set `self.UpgradeSuccess` false))
              (return _output_get_11))))
        (:`NewEnumerator2`
          (if (<= _lavabomberlevel3 _currentsouls_5)
            (`/Game/Jake-Towers/BP_Currency.RemoveSouls` (`/Game/Blueprints/Gameplay/BP_GameManager.BP_Currency` (`self.GM_Ref`)) _lavabomberlevel3)
            (bind _result_11 (`/Engine/EditorBlueprintResources/StandardMacros.IncrementInt` (`self.TowerLevel`))
              (:`  `
                (set `self.TowerLevel` _result_11)
                (goto _label)))
            (else
              (bind _output_get_12 (set `self.UpgradeSuccess` false))
              (return _output_get_12))))
        (:`NewEnumerator3`
          (if (<= _implevel3 _currentsouls_5)
            (`/Game/Jake-Towers/BP_Currency.RemoveSouls` (`/Game/Blueprints/Gameplay/BP_GameManager.BP_Currency` (`self.GM_Ref`)) _implevel3)
            (bind _result_12 (`/Engine/EditorBlueprintResources/StandardMacros.IncrementInt` (`self.TowerLevel`))
              (:`  `
                (set `self.TowerLevel` _result_12)
                (goto _label)))
            (else
              (bind _output_get_13 (set `self.UpgradeSuccess` false))
              (return _output_get_13))))))
    (:`4`
      (`KismetSystemLibrary.PrintString` "Max Level"))))

(fn `UserConstructionScript`)